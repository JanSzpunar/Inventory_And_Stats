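; Base interactable actor that shows a screen-space prompt while selected and provides an Interact event, which here only prints a debug string.
; On BeginPlay it sets every static mesh under Meshes to ignore the Camera collision channel.
; Selected creates a widget component at InteractionWidget's relative location, hosting a WBP_InteractionPrompt with InteractText.
; Deselected destroys that component, so the prompt exists only during selection.
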(event `self.ReceiveBeginPlay`
  (`parent.ReceiveBeginPlay`)
  (for _array_element (`SceneComponent.GetChildrenComponents` (`self.Meshes`) true)
    (bind _asstatic_mesh_component (cast `StaticMeshComponent` _array_element))
    (`PrimitiveComponent.SetCollisionResponseToChannel` _asstatic_mesh_component "ECC_Camera" "ECR_Ignore")))

(event `SelectionInterface.Selected`
  (bind _returnvalue (`|AddComponentByClass` "/Script/UMG.WidgetComponent" false (`KismetMathLibrary.MakeTransform` (`SceneComponent.RelativeLocation` (`self.InteractionWidget`)))))
  (bind _output_get (set `self.Prompt` _returnvalue))
  (`PrimitiveComponent.SetCollisionEnabled` _output_get "NoCollision")
  (`WidgetComponent.SetDrawAtDesiredSize` _output_get true)
  (bind _returnvalue_2 (`|CreateWidget` "/Game/HUD/Interactables/WBP_InteractionPrompt.WBP_InteractionPrompt_C" null (`self.interactText`)))
  (`WidgetComponent.SetWidget` _output_get _returnvalue_2)
  (`WidgetComponent.SetWidgetSpace` _output_get "Screen")
  (`WidgetComponent.SetPivot` _output_get (0.5 0.5)))

(event `SelectionInterface.Deselected`
  (bind _prompt (`self.Prompt`)
    (:`then`
      (`ActorComponent.K2_DestroyComponent` _prompt))
    (:`else`)))

(event `InteractableInterface.Interact`
  (params (Interactor :type "Actor Object Reference"))
  (`KismetSystemLibrary.PrintString` "Interact"))

(fn `UserConstructionScript`)