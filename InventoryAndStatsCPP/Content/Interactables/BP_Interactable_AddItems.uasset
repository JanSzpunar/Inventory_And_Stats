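; Interactable actor that gives the player items from the DT_Items data table, apparently for testing the inventory.
; Each Interact call adds one of the item at the current row index to the Player inventory through a GameState message.
; The index advances only when the add succeeds and wraps to the first row once it runs past the table's end.
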(event `InteractableInterface.Interact`
  (params (Interactor :type "Actor Object Reference"))
  (bind _outrownames (`DataTableFunctionLibrary.GetDataTableRowNames` "/Game/Inventory/DT_Items.DT_Items"))
  (if (not (`KismetArrayLibrary.Array_IsValidIndex` _outrownames (`self.CurrentItemIndex`)))
    (set `self.CurrentItemIndex` 0))
  (bind _output (`|GetArrayItem` _outrownames (`self.CurrentItemIndex`)))
  (`|GetDataTableRow` "/Game/Inventory/DT_Items.DT_Items" _output
    (:`then`
      (bind _returnvalue (message `InventoryInterface.AddItemToInventory` (`GameplayStatics.GetGameState`) "Player" (make `InventoryItem` _output (make `InventoryItemDynamic` 1))))
      (if (break `AddItemResult` _returnvalue)
        (`/Engine/EditorBlueprintResources/StandardMacros.IncrementInt` (`self.CurrentItemIndex`))))))

(fn `UserConstructionScript`
  (`parent.UserConstructionScript`))