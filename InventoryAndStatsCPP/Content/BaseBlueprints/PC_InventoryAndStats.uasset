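; Player controller Blueprint that maps Enhanced Input actions to inventory, character panel, character switching and interaction.
; The inventory and character panel inputs send messages to the HUD to switch those screens, with "Player" identifying the inventory.
; Character selection cycles to the next controlled character.
; Interact takes the current interactable from InteractableController and, if valid, sends it an interact message carrying the currently controlled character.
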(event `EnhancedInput|/Game/Input/Actions/IA_Inventory`
  (params (ActionValue :type Boolean) (ElapsedSeconds :type "Float (double-precision)") (TriggeredSeconds :type "Float (double-precision)") (InputAction :type "InputAction Object Reference" :default "/Game/Input/Actions/IA_Inventory.IA_Inventory"))
  (:`Started`
    (message `InventoryHUDInterface.SwitchInventory` (`self.GetHUD`) "Player")))

(event `EnhancedInput|/Game/Input/Actions/IA_SelectCharacter`
  (params (ActionValue :type Boolean) (ElapsedSeconds :type "Float (double-precision)") (TriggeredSeconds :type "Float (double-precision)") (InputAction :type "InputAction Object Reference" :default "/Game/Input/Actions/IA_SelectCharacter.IA_SelectCharacter"))
  (:`Started`
    (`CharactersControllerInterface.SelectNextControlledCharacter`)))

(event `EnhancedInput|/Game/Input/Actions/IA_CharacterPanel`
  (params (ActionValue :type Boolean) (ElapsedSeconds :type "Float (double-precision)") (TriggeredSeconds :type "Float (double-precision)") (InputAction :type "InputAction Object Reference" :default "/Game/Input/Actions/IA_CharacterPanel.IA_CharacterPanel"))
  (:`Started`
    (message `CharacterPanelHUDInterface.SwitchCharacterPanel` (`self.GetHUD`))))

(event `EnhancedInput|/Game/Input/Actions/IA_Interact`
  (params (ActionValue :type Boolean) (ElapsedSeconds :type "Float (double-precision)") (TriggeredSeconds :type "Float (double-precision)") (InputAction :type "InputAction Object Reference" :default "/Game/Input/Actions/IA_Interact.IA_Interact"))
  (bind _returnvalue (`InteractableController.GetCurrentInteractable` (`self.InteractableController`)))
  (:`Started`
    (`/Engine/EditorBlueprintResources/StandardMacros.IsValid` _returnvalue
      (:`Is Valid`
        (bind _returnvalue_2 (`CharactersControllerInterface.GetCurrentlyControlledCharacter`))
        (message `InteractableInterface.Interact` _returnvalue _returnvalue_2)))))

(fn `UserConstructionScript`)