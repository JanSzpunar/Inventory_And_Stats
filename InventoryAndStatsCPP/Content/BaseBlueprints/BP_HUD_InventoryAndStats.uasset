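; BP_HUD_InventoryAndStats creates the main HUD widget and manages opening, closing and toggling of inventory windows and the character panel.
; Open inventories are tracked in a map, with "Player" placed in the main slot and others in the additional slot.
; Opening shows the cursor with Game-and-UI input.
; Closing an inventory restores game-only input immediately, whereas closing the character panel does so only when no inventories remain.
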(event `self.ReceiveBeginPlay`
  (bind _returnvalue (`|CreateWidget` "/Game/HUD/WBP_HUD.WBP_HUD_C"))
  (bind _output_get (set `self.HUD` _returnvalue))
  (`UserWidget.AddToViewport` _output_get 0))

(event `InventoryHUDInterface.CloseInventory`
  (params (Inventory :type Name))
  (bind _returnvalue (`GameplayStatics.GetPlayerController` 0))
  (bind (_value _returnvalue_2) (`BlueprintMapLibrary.Map_Find` (`self.inventories`) Inventory))
  (if _returnvalue_2
    (`/Engine/EditorBlueprintResources/StandardMacros.IsValid` _value
      (:`Is Valid`
        (`Widget.RemoveFromParent` _value)
        (`|ExecutionSequence`
          (:`then_0`
            (`WidgetBlueprintLibrary.SetInputMode_GameOnly` _returnvalue)
            (set `PlayerController.bShowMouseCursor` false _returnvalue))
          (:`then_1`
            (`BlueprintMapLibrary.Map_Remove` (`self.inventories`) Inventory :!label _label))))
      (:`Is Not Valid`
        (goto _label)))))

(event `InventoryHUDInterface.OpenInventory`
  (params (Inventory :type Name))
  (bind _hud (`self.HUD`))
  (`self.CloseInventory` Inventory)
  (bind _returnvalue (`|CreateWidget` "/Game/HUD/Inventory/WBP_Inventory.WBP_Inventory_C" null Inventory))
  (`PanelWidget.AddChild` (select `bool` (== Inventory "Player") :`false` (`/Game/HUD/WBP_HUD.AdditionalInventory` _hud) :`true` (`/Game/HUD/WBP_HUD.Inventory` _hud) :!type "PanelWidget Object Reference") _returnvalue)
  (`BlueprintMapLibrary.Map_Add` (`self.inventories`) Inventory _returnvalue)
  (`WidgetBlueprintLibrary.SetInputMode_GameAndUIEx` (`GameplayStatics.GetPlayerController` 0) _returnvalue)
  (set `PlayerController.bShowMouseCursor` true (`GameplayStatics.GetPlayerController` 0)))

(event `InventoryHUDInterface.SwitchInventory`
  (params (Inventory :type Name))
  (bind (_value _returnvalue) (`BlueprintMapLibrary.Map_Find` (`self.inventories`) Inventory))
  (if _returnvalue
    (`/Engine/EditorBlueprintResources/StandardMacros.IsValid` _value
      (:`Is Valid`
        (`self.CloseInventory` Inventory))
      (:`Is Not Valid`
        (`self.OpenInventory` Inventory :!label _label_2)))
    (else
      (goto _label_2))))

(event `CharacterPanelHUDInterface.SwitchCharacterPanel`
  (`/Engine/EditorBlueprintResources/StandardMacros.IsValid` (`self.characterPanel`)
    (:`Is Valid`
      (`CharacterPanelHUDInterface.CloseCharacterPanel`))
    (:`Is Not Valid`
      (`CharacterPanelHUDInterface.OpenCharacterPanel`))))

(event `CharacterPanelHUDInterface.OpenCharacterPanel`
  (`CharacterPanelHUDInterface.CloseCharacterPanel`)
  (bind _returnvalue (`|CreateWidget` "/Game/HUD/CharacterPanel/WBP_CharacterPanel.WBP_CharacterPanel_C"))
  (bind _output_get (set `self.characterPanel` _returnvalue))
  (`PanelWidget.AddChild` (`/Game/HUD/WBP_HUD.CharacterPanel` (`self.HUD`)) _output_get)
  (add `/Game/HUD/CharacterPanel/WBP_CharacterPanel.OnCharacterPanelCloseRequested` (`self.characterPanel`) (delegate `OnCharacterPanelCloseRequested_Event`))
  (`WidgetBlueprintLibrary.SetInputMode_GameAndUIEx` (`GameplayStatics.GetPlayerController` 0) (`self.characterPanel`))
  (set `PlayerController.bShowMouseCursor` true (`GameplayStatics.GetPlayerController` 0)))

(event `OnCharacterPanelCloseRequested_Event`
  (`CharacterPanelHUDInterface.CloseCharacterPanel`))

(event `CharacterPanelHUDInterface.CloseCharacterPanel`
  (bind _returnvalue (`GameplayStatics.GetPlayerController` 0))
  (`/Engine/EditorBlueprintResources/StandardMacros.IsValid` (`self.characterPanel`)
    (:`Is Valid`
      (`Widget.RemoveFromParent` (`self.characterPanel`))
      (set `self.characterPanel` null)
      (if (`BlueprintMapLibrary.Map_IsEmpty` (`self.inventories`))
        (`WidgetBlueprintLibrary.SetInputMode_GameOnly` _returnvalue)
        (set `PlayerController.bShowMouseCursor` false _returnvalue)))))

(event `CharacterPanelHUDInterface.RefreshCharacterPanel`
  (bind _characterpanel (`self.characterPanel`)
    (:`then`
      (`HUDInterface.Refresh` _characterpanel))
    (:`else`)))

(fn `UserConstructionScript`)